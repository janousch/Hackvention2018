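; BP_Podium is a display podium that provides a sculptable anatomy mesh for the VR pawn.
; The construction script previews the configured mesh, transform and materials on the podium.
; On BeginPlay it spawns a BP_SculptingMesh with that mesh at the preview's world transform, then destroys the preview component.
; When a BP_PawnVR overlaps the Box, the podium assigns its sculpting mesh to that pawn.
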(event OnComponentBeginOverlap(Box)
  (params (OverlappedComponent :type Primitive%20Component%20Object%20Reference) (OtherActor :type Actor%20Object%20Reference) (OtherComp :type Primitive%20Component%20Object%20Reference) (OtherBodyIndex :type Integer) (bFromSweep :type Boolean) (SweepResult :type Hit%20Result%20Structure%20%28by%20ref%29))
  (bind _asbp_pawn_vr (Utilities|Casting|CastToBP_PawnVR OtherActor))
  (Variables|/Game/Blueprints/Player/BP_PawnVR.BP_PawnVR_C|SetSculptingMesh _asbp_pawn_vr (Variables|Default|GetSculptingMesh)))

(event EventBeginPlay
  (bind _returnvalue (Game|SpawnActorfromClass "/Game/Blueprints/BP_SculptingMesh.BP_SculptingMesh_C" (Math|Transform|MakeTransform (Transformation|GetActorLocation) "0, 0, 0" "1,1,1") "AlwaysSpawn" 0 (Variables|Default|GetMesh) (Transformation|GetWorldTransform (Variables|Default|GetAnatomyMesh)) 0))
  (Variables|Default|SetSculptingMesh _returnvalue)
  (Components|DestroyComponent (Variables|Default|GetAnatomyMesh)))

(fn ConstructionScript
  (bind _anatomymesh (Variables|Default|GetAnatomyMesh))
  (Components|StaticMesh|SetStaticMesh _anatomymesh (Variables|Default|GetMesh))
  (Transformation|SetRelativeTransform _anatomymesh (Variables|Default|GetMeshTransform) false false)
  (Rendering|Material|SetMaterial (Variables|Default|GetPodium) 0 (Variables|Default|GetPodiumMaterial))
  (Rendering|Material|SetMaterial (Variables|Default|GetAnatomyMesh) 0 "/Game/Materials/M_Plastic.M_Plastic"))