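; BP_SculptingMesh is a sculpting actor that grows by adding sphere or cube procedural mesh pieces.
; The construction script caches vertices and triangles from the sphere and cube static meshes.
; Extend calls ExtendHelper, which adds a uniformly scaled ProceduralMeshComponent, builds its section from the chosen form and applies the material.
; Extend passes no location to the helper, and Reduce is an empty stub.
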(event Custom|Extend
  (params (Scaling :type Float%20%28single-precision%29) (Form :type ESculptExtendForm%20Enum :default "NewEnumerator0") (Material :type Material%20Interface%20Object%20Reference))
  (CallFunction|ExtendHelper "0, 0, 0" Scaling Form Material))

(event Custom|Reduce)

(fn ConstructionScript
  (Utilities|FlowControl|Sequence
    (:then_0
      (bind (_vertices _triangles) (Class|KismetProceduralMeshLibrary|GetSectionfromStaticMesh "/Game/Ressources/StarterContent/Shapes/Shape_Sphere.Shape_Sphere"))
      (Variables|Default|SetSphereVertices _vertices)
      (Variables|Default|SetSphereTriangles _triangles))
    (:then_1
      (bind (_vertices_2 _triangles_2) (Class|KismetProceduralMeshLibrary|GetSectionfromStaticMesh "/Game/Ressources/StarterContent/Shapes/Shape_Cube.Shape_Cube"))
      (Variables|Default|SetCubeVertices _vertices_2)
      (Variables|Default|SetCubeTriangles _triangles_2))))

(fn ExtendHelper
  (params (Location :type Vector) (Scaling :type Float%20%28single-precision%29) (Form :type ESculptExtendForm%20Enum :default "NewEnumerator0") (Material :type Material%20Interface%20Object%20Reference))
  (LocalVariables|SetCurrentForm Form)
  (LocalVariables|SetCurrentMaterial Material)
  (bind _returnvalue (AddComponent|AddProceduralMeshComponent false (Math|Transform|MakeTransform Location "0, 0, 0" (Math|Vector|MakeVector Scaling Scaling Scaling))))
  (LocalVariables|SetNewMeshComponent _returnvalue)
  (switch Utilities|FlowControl|Switch|SwitchonESculptExtendForm (LocalVariables|GetCurrentForm)
    (:NewEnumerator0
      (Class|ProceduralMeshComponent|CreateMeshSectionLinearColor (LocalVariables|GetNewMeshComponent) 0 (Variables|Default|GetSphereVertices) (Variables|Default|GetSphereTriangles) 0 0 0 0 false))
    (:NewEnumerator1
      (Class|ProceduralMeshComponent|CreateMeshSectionLinearColor (LocalVariables|GetNewMeshComponent) 0 (Variables|Default|GetCubeVertices) (Variables|Default|GetCubeTriangles) 0 0 0 0 false)))
  (Rendering|Material|SetMaterial (LocalVariables|GetNewMeshComponent) 0 (LocalVariables|GetCurrentMaterial)))